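; BP_Note1 is a note actor, apparently for a rhythm mechanic, that travels along the Lane01 spline of BP_Spline.
; On BeginPlay it finds and caches the spline actor; MoveNotes plays a timeline with its rate scaled by TimeToComplete.
; Each update lerps distance along the spline and sets the actor's transform from local-space spline location and rotation, using the Cube's relative scale.
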(event `self.ReceiveBeginPlay`
  (bind _returnvalue (`GameplayStatics.GetActorOfClass` "/Game/ParkourLevel/BP_Spline.BP_Spline_C"))
  (set `self.Rhythm Spline` _returnvalue))

(event `MoveNotes`
  (bind _lane_01 (`/Game/ParkourLevel/BP_Spline.Lane_01` (`self.Rhythm Spline`)))
  (`TimelineComponent.SetPlayRate` (`self.Timeline`) (/ 1.0 (`self.Time To Complete`)))
  (bind (_direction _newtrack_0) (`Timeline|Timeline` :!via `PlayFromStart`)
    (:`Update`
      (bind _returnvalue (`KismetMathLibrary.Lerp` 0.0 (`SplineComponent.GetSplineLength` (`/Game/ParkourLevel/BP_Spline.Lane_01` (`self.Rhythm Spline`))) _newtrack_0))
      (`self.K2_SetActorTransform` (`KismetMathLibrary.MakeTransform` (`SplineComponent.GetLocationAtDistanceAlongSpline` _lane_01 _returnvalue "Local") (`SplineComponent.GetRotationAtDistanceAlongSpline` _lane_01 _returnvalue "Local") (`SceneComponent.RelativeScale3D` (`self.Cube`)))))))

(fn `UserConstructionScript`)