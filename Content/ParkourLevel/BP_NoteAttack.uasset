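; BP_NoteAttack is a cube-based attack actor that travels along the Lane01 spline of the level's BP_SplineAttack.
; BeginPlay caches that spline actor and sets the cube's height.
; MoveAttack plays a timeline at a rate of 1/TimeToComplete, mapping its track to spline distance to drive actor location and rotation in the spline's local space.
; A RandomiseZ helper returns a grid-snapped random height offset, unused in these graphs.
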(event `self.ReceiveBeginPlay`
  (bind _returnvalue (`GameplayStatics.GetActorOfClass` "/Game/ParkourLevel/BP_SplineAttack.BP_SplineAttack_C"))
  (set `self.Rhythm Spline` _returnvalue)
  (`SceneComponent.K2_SetRelativeLocation` (`self.Cube`) (0.0 0.0 80.0) false false))

(event `MoveAttack`
  (bind _rhythm_spline (`self.Rhythm Spline`))
  (`TimelineComponent.SetPlayRate` (`self.Timeline`) (/ 1.0 (`self.Time To Complete`)))
  (bind (_direction _newtrack_0) (`Timeline|Timeline` :!via `PlayFromStart`)
    (:`Update`
      (bind _returnvalue (`KismetMathLibrary.Lerp` 0.0 (`SplineComponent.GetSplineLength` (`/Game/ParkourLevel/BP_SplineAttack.Lane_01` (`self.Rhythm Spline`))) _newtrack_0))
      (`self.K2_SetActorTransform` (`KismetMathLibrary.MakeTransform` (`SplineComponent.GetLocationAtDistanceAlongSpline` (`/Game/ParkourLevel/BP_SplineAttack.Lane_01` _rhythm_spline) _returnvalue "Local") (`SplineComponent.GetRotationAtDistanceAlongSpline` (`/Game/ParkourLevel/BP_SplineAttack.Lane_01` _rhythm_spline) _returnvalue "Local") (`SceneComponent.RelativeScale3D` (`self.Cube`)))))))

(fn `RandomiseZ`
  (returns (ReturnValue :type "Vector Structure"))
  (bind (_relativelocation_x _relativelocation_y _relativelocation_z) (`KismetMathLibrary.BreakVector` (`SceneComponent.RelativeLocation` (`self.Cube`))))
  (return (`KismetMathLibrary.MakeVector` _relativelocation_x _relativelocation_y (`KismetMathLibrary.GridSnap_Float` (+ _relativelocation_z (`KismetMathLibrary.RandomFloatInRange` 0.0 400.0)) 50.0))))

(fn `UserConstructionScript`)