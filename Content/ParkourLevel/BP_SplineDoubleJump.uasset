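; BP_SplineDoubleJump is a music-driven spawner for double jump notes in the parkour level.
; It adds an audio component on BeginPlay and watches its MetaSound "DoubleJumpCue" output as a beat trigger.
; Each cue change spawns a BP_NoteDoubleJump at the Spawner's relative location and calls MoveNotes on it.
; The Destroyer overlap box destroys any actor that enters it.
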(event `self.ReceiveBeginPlay`
  (bind _returnvalue (`AddComponent|NODE_AddAudioComponent-3`))
  (`MetaSoundOutputSubsystem.WatchOutput` (subsystem `MetaSoundOutputSubsystem`) _returnvalue "DoubleJumpCue" (delegate `CueChange`) "None" "None"))

(event `CueChange`
  (params (OutputName :type Name) (Output :type "MetaSoundOutput Structure (by ref)"))
  ; Beat trigger
  (`KismetSystemLibrary.PrintString` "DoubleJump")
  (bind _returnvalue (`|SpawnActorFromClass` "/Game/ParkourLevel/BP_NoteDoubleJump.BP_NoteDoubleJump_C" (`KismetMathLibrary.MakeTransform` (`SceneComponent.RelativeLocation` (`self.Spawner`))) "Undefined" "MultiplyWithRoot" null null))
  (`/Game/ParkourLevel/BP_NoteDoubleJump.MoveNotes` _returnvalue))

(event `self.Destroyer.OnComponentBeginOverlap`
  (params (OverlappedComponent :type "PrimitiveComponent Object Reference") (OtherActor :type "Actor Object Reference") (OtherComp :type "PrimitiveComponent Object Reference") (OtherBodyIndex :type Integer) (bFromSweep :type Boolean) (SweepResult :type "HitResult Structure (by ref)"))
  ; destroy box
  (`self.K2_DestroyActor` OtherActor))

(fn `UserConstructionScript`)