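; BP_NoteDoubleJump is an asteroid "note" obstacle that calls DoDamage on the third-person character when overlapped.
; On BeginPlay it finds the BP_SplineDoubleJump actor and lowers the asteroid component.
; MoveNotes plays a timeline scaled by TimeToComplete, moving the actor along that spline's Lane01 using local-space position and rotation as its transform.
; A grid-snapped random height helper, RandomiseZ, exists but is unused.
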(event `self.Astroid.OnComponentBeginOverlap`
  (params (OverlappedComponent :type "PrimitiveComponent Object Reference") (OtherActor :type "Actor Object Reference") (OtherComp :type "PrimitiveComponent Object Reference") (OtherBodyIndex :type Integer) (bFromSweep :type Boolean) (SweepResult :type "HitResult Structure (by ref)"))
  (bind _asbp_third_person_character (cast `/Game/ThirdPerson/Blueprints/BP_ThirdPersonCharacter` OtherActor))
  (`/Game/ThirdPerson/Blueprints/BP_ThirdPersonCharacter.DoDamage` _asbp_third_person_character))

(event `self.ReceiveBeginPlay`
  (bind _returnvalue (`GameplayStatics.GetActorOfClass` "/Game/ParkourLevel/BP_SplineDoubleJump.BP_SplineDoubleJump_C"))
  (set `self.Rhythm Spline` _returnvalue)
  (`SceneComponent.K2_SetRelativeLocation` (`self.Astroid`) (0.0 0.0 -50.0) false false))

(event `MoveNotes`
  (bind _lane_01 (`/Game/ParkourLevel/BP_SplineDoubleJump.Lane_01` (`self.Rhythm Spline`)))
  (`TimelineComponent.SetPlayRate` (`self.Timeline`) (/ 1.0 (`self.Time To Complete`)))
  (bind (_direction _newtrack_0) (`Timeline|Timeline` :!via `PlayFromStart`)
    (:`Update`
      (bind _returnvalue (`KismetMathLibrary.Lerp` 0.0 (`SplineComponent.GetSplineLength` (`/Game/ParkourLevel/BP_SplineDoubleJump.Lane_01` (`self.Rhythm Spline`))) _newtrack_0))
      (`self.K2_SetActorTransform` (`KismetMathLibrary.MakeTransform` (`SplineComponent.GetLocationAtDistanceAlongSpline` _lane_01 _returnvalue "Local") (`SplineComponent.GetRotationAtDistanceAlongSpline` _lane_01 _returnvalue "Local") (`SceneComponent.RelativeScale3D` (`self.Astroid`)))))))

(fn `RandomiseZ`
  (returns (ReturnValue :type "Vector Structure"))
  (bind (_relativelocation_x _relativelocation_y _relativelocation_z) (`KismetMathLibrary.BreakVector` (`SceneComponent.RelativeLocation` (`self.Astroid`))))
  (return (`KismetMathLibrary.MakeVector` _relativelocation_x _relativelocation_y (`KismetMathLibrary.GridSnap_Float` (+ _relativelocation_z (`KismetMathLibrary.RandomFloatInRange` 0.0 400.0)) 50.0))))

(fn `UserConstructionScript`)