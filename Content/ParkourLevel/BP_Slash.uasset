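; BP_Slash is a short-lived slash attack actor that destroys note attacks it touches.
; On BeginPlay it activates the NEAttack04 effect, waits briefly, prints a give or take points message based on HitAlien, then destroys itself.
; The capsule overlap destroys any BP_NoteAttack it meets and sets HitAlien.
; Scoring is only debug prints, and the Slash event is empty.
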(event `self.ReceiveBeginPlay`
  (`ActorComponent.Activate` (`self.NE_attack04`) false)
  (`KismetSystemLibrary.Delay` 0.5)
  (if (`self.HitAlien`)
    (`KismetSystemLibrary.PrintString` "Give Points")
    (else
      (`KismetSystemLibrary.PrintString` "Take Points")))
  (`self.K2_DestroyActor`))

(event `self.ReceiveTick`
  (params (DeltaSeconds :type "Float (single-precision)")))

(event `Slash`)

(event `self.Capsule.OnComponentBeginOverlap`
  (params (OverlappedComponent :type "PrimitiveComponent Object Reference") (OtherActor :type "Actor Object Reference") (OtherComp :type "PrimitiveComponent Object Reference") (OtherBodyIndex :type Integer) (bFromSweep :type Boolean) (SweepResult :type "HitResult Structure (by ref)"))
  (if (== (`GameplayStatics.GetObjectClass` OtherActor) "/Game/ParkourLevel/BP_NoteAttack.BP_NoteAttack_C")
    (`self.K2_DestroyActor` OtherActor)
    (set `self.HitAlien` true)))

(fn `UserConstructionScript`)